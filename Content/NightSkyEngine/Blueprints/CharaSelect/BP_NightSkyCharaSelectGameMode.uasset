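; Game mode for the NightSkyEngine character select screen that builds its UI on BeginPlay.
; It clears existing widgets, creates a shared WBP_Base for player one's controller and pushes the WBP_CSelectGrid menu onto it.
; Both player controllers receive that base as UIBase and switch to UI-only input, player one after a two-tick delay and player two only if that controller exists.
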(event EventBeginPlay
  (bind _returnvalue (Game|GetPlayerController 1))
  (Viewport|RemoveAllWidgets)
  (bind _asbp_chara_select_player_controller (Utilities|Casting|CastToBP_CharaSelectPlayerController (Game|GetPlayerController 0)))
  (bind _returnvalue_2 (UserInterface|CreateWidget "/Game/NightSkyEngine/UI/Common/WBP_Base.WBP_Base_C" _asbp_chara_select_player_controller))
  (UserInterface|Viewport|AddtoViewport _returnvalue_2 0)
  (Default|PushMenu _returnvalue_2 "/Game/NightSkyEngine/UI/CharaSelect/WBP_CSelectGrid.WBP_CSelectGrid_C")
  (Variables|/Game/NightSkyEngine/Blueprints/Menu/BP_MenuPlayerController.BP_MenuPlayerController_C|SetUIBase _asbp_chara_select_player_controller _returnvalue_2)
  (Utilities|FlowControl|DelayUntilNextTick)
  (Utilities|FlowControl|DelayUntilNextTick)
  (Input|SetInputModeUIOnly _asbp_chara_select_player_controller 0 "DoNotLock" false)
  (Utilities|IsValid _returnvalue
    (:Is%20Valid
      (bind _asbp_chara_select_player_controller_2 (Utilities|Casting|CastToBP_CharaSelectPlayerController _returnvalue)
        (:then
          (Variables|/Game/NightSkyEngine/Blueprints/Menu/BP_MenuPlayerController.BP_MenuPlayerController_C|SetUIBase _asbp_chara_select_player_controller_2 _returnvalue_2)
          (Input|SetInputModeUIOnly _asbp_chara_select_player_controller_2 0 "DoNotLock" false))
        (:CastFailed
          (Development|PrintString "can't Cast"))))
    (:Is%20Not%20Valid
      (Development|PrintString "No Controller"))))

(event EventTick
  (params (DeltaSeconds :type Float%20%28single-precision%29)))

(fn ConstructionScript)