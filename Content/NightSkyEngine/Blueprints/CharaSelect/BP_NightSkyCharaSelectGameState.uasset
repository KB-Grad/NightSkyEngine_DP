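; Game state for the NightSky character select screen that sets up local players and gathers selectable character and stage data.
; BeginPlay initializes the game instance's player list, then a tick later creates a second local player if needed outside training, CPU battle and multiplayer.
; GatherCharaData and GatherStageData synchronously load primary assets into arrays; only the stage list is cleared first.
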(event EventBeginPlay
  (bind _asbp_night_sky_game_instance (Utilities|Casting|CastToBP_NightSkyGameInstance (Game|GetGameInstance)))
  (Default|InitPlayerList _asbp_night_sky_game_instance)
  (bind _asbp_night_sky_game_instance_2 (Utilities|Casting|CastToBP_NightSkyGameInstance (Game|GetGameInstance)))
  (Utilities|FlowControl|DelayUntilNextTick)
  (if (and (and (not (or (Variables|/Script/NightSkyEngine.NightSkyGameInstance|GetIsTraining _asbp_night_sky_game_instance_2) (Variables|/Script/NightSkyEngine.NightSkyGameInstance|GetIsCPUBattle _asbp_night_sky_game_instance_2))) (Utilities|Enum|NotEqual(Enum) (Variables|/Script/NightSkyEngine.NightSkyGameInstance|GetFighterRunner _asbp_night_sky_game_instance_2) "Multiplayer")) (< (Class|GameplayStatics|GetNumLocalPlayerControllers) 2))
    (Class|GameplayStatics|CreatePlayer -1)))

(fn ConstructionScript)

(fn GatherCharaData
  (bind _outprimaryassetidlist (Class|KismetSystemLibrary|GetPrimaryAssetIdList "PrimaryCharaData"))
  (for _array_element _outprimaryassetidlist
    (bind _returnvalue (Utilities|LoadAssetBlocking (Class|KismetSystemLibrary|GetSoftObjectReferencefromPrimaryAssetId _array_element)))
    (bind _asprimary_chara_data (Utilities|Casting|CastToPrimaryCharaData _returnvalue))
    (Utilities|Array|Add (Variables|Default|GetCharaDatas) _asprimary_chara_data)))

(fn GatherStageData
  (Utilities|Array|Clear (Variables|Default|GetStageDatas))
  (bind _outprimaryassetidlist (Class|KismetSystemLibrary|GetPrimaryAssetIdList "PrimaryStageData"))
  (for _array_element _outprimaryassetidlist
    (bind _returnvalue (Utilities|LoadAssetBlocking (Class|KismetSystemLibrary|GetSoftObjectReferencefromPrimaryAssetId _array_element)))
    (bind _asprimary_stage_data (Utilities|Casting|CastToPrimaryStageData _returnvalue))
    (Utilities|Array|Add (Variables|Default|GetStageDatas) _asprimary_stage_data)))