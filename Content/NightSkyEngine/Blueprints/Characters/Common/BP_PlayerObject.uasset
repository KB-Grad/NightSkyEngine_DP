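; Common player character Blueprint for NightSkyEngine that handles material setup and the meter reset at round start.
; One tick after BeginPlay, it calls SetColor, an empty function here, then SetupMaterials.
; SetupMaterials matches child mesh components to MaterialData entries by name, creating dynamic instances for material slots and overlays.
; Round init spends the full meter, then refills it to a quarter one tick later.
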(event EventBeginPlay
  (Utilities|FlowControl|DelayUntilNextTick)
  (CallFunction|SetColor)
  (CallFunction|SetupMaterials))

(event EventRoundInitBP
  (bind _maxmeter (Variables|Default|GetMaxMeter))
  (Class|PlayerObject|UseMeter _maxmeter)
  (Utilities|FlowControl|DelayUntilNextTick)
  (Class|PlayerObject|AddMeter (/ _maxmeter 4)))

(fn ConstructionScript)

(fn SetColor)

(fn SetupMaterials
  (bind _materialdata (Variables|Default|GetMaterialData))
  (Utilities|IsValid _materialdata
    (:Is%20Valid
      (for _array_element (Components|GetChildrenComponents (Variables|Transformation|GetRootComponent) true)
        (bind _asmesh_component (Utilities|Casting|CastToMeshComponent _array_element))
        (bind _array_element_2 (Utilities|Array|ForEachLoopwithBreak (Variables|/Script/NightSkyEngine.MaterialData|GetMaterialStructs _materialdata) :!label _label)
          (:LoopBody
            (if (Utilities|Enum|Equal(Enum) (Utilities|GetObjectName _array_element) (Utilities|String|ToString(Name) (.Name (Utilities|Struct|BreakMaterialStruct _array_element_2))))
              (for (_array_element_3 _array_index) (.Material (Utilities|Struct|BreakMaterialStruct _array_element_2))
                (Rendering|Material|CreateDynamicMaterialInstance _asmesh_component _array_index _array_element_3 "None" :!class /Script/Engine.PrimitiveComponent))
              (goto _label Break)))
          (:Completed
            (bind _returnvalue (Rendering|Material|CreateDynamicMaterialInstance (.OverlayMaterial (Utilities|Struct|BreakMaterialStruct _array_element_2)) "None" "None" :!class /Script/Engine.KismetMaterialLibrary))
            (Rendering|Material|SetOverlayMaterial _asmesh_component _returnvalue :!class /Script/Engine.MeshComponent)))))))