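; Knight character Blueprint for a NightSkyEngine game, adding the character's weapon and color variants on top of its parent class.
; The construction script attaches the greatsword mesh to the body's right-hand weapon socket, keeping relative transforms.
; SetColor calls the parent, then picks one of two Knight material data assets from the color index.
; The event graph holds no active logic.
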(event EventBeginPlay
  (|CallParentFunction) ; This node is disabled and will not be called.\nDrag off pins to build functionality.
)

(event Collision|EventActorBeginOverlap
  (params (OtherActor :type Actor%20Object%20Reference)))

(event EventTick
  (params (DeltaSeconds :type Float%20%28single-precision%29)))

(fn ConstructionScript
  (|CallParentFunction)
  (Transformation|AttachComponentToComponent (Variables|Default|GetGreatsword_SM) (Variables|Default|GetBody) "weapon_r" "KeepRelative" "KeepRelative" "KeepRelative" true))

(fn SetColor
  (|CallParentFunction)
  (switch int (Variables|Default|GetColorIndex)
    (:1
      (Variables|Default|SetMaterialData "/Game/NightSkyEngine/CharacterAssets/Knight/Materials/Color1/DA_KnightMaterials01.DA_KnightMaterials01"))
    (:2
      (Variables|Default|SetMaterialData "/Game/NightSkyEngine/CharacterAssets/Knight/Materials/Color2/DA_KnightMaterials02.DA_KnightMaterials02"))))