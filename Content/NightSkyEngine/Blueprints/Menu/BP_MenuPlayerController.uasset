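; BP_MenuPlayerController is the menu player controller, handling UI navigation and online lobby hosting and searching.
; On BeginPlay it binds the session search callback and adds the menu input mapping a frame later.
; Push events forward prompts, menus and modals to UIBase.
; Host and Join set the fighter runner to Multiplayer; Host opens a listen-server level, while Join clears and refills the lobby list from found sessions.
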(event Custom|PushPrompt
  (params (PromptText :type Text) (PromptOwner :type WBP%20Base%20Activatable%20Widget%20Object%20Reference) (PromptIndex :type Integer))
  (Default|PushPrompt (Variables|Default|GetUIBase) PromptText PromptOwner PromptIndex))

(event Custom|OnFindSessionsCompleteEvent
  (params (SessionResults :type Array%20of%20NSE%20Session%20Info%20Structures) (bSuccess :type Boolean))
  (if bSuccess
    (bind _foundwidgets (Widget|GetAllWidgetsOfClass "/Game/NightSkyEngine/UI/Online/WBP_LobbyList.WBP_LobbyList_C" false))
    (for _array_element SessionResults
      (bind _returnvalue (UserInterface|CreateWidget "/Game/NightSkyEngine/UI/Online/WBP_LobbyItem.WBP_LobbyItem_C" self _array_element))
      (Widget|Panel|AddChild (Variables|/Game/NightSkyEngine/UI/Online/WBP_LobbyList.WBP_LobbyList_C|GetLobbyList (Utilities|Array|Get(acopy) _foundwidgets)) _returnvalue))))

(event Custom|HostGame
  (bind _asbp_night_sky_game_instance (Utilities|Casting|CastToBP_NightSkyGameInstance (Game|GetGameInstance)))
  (Variables|/Script/NightSkyEngine.NightSkyGameInstance|SetFighterRunner _asbp_night_sky_game_instance "Multiplayer")
  (Game|OpenLevel(byObjectReference) "/Game/NightSkyEngine/Maps/Connecting_PL.Connecting_PL" true "listen"))

(event Custom|JoinGame
  (bind _asbp_night_sky_game_instance (Utilities|Casting|CastToBP_NightSkyGameInstance (Game|GetGameInstance)))
  (Variables|/Script/NightSkyEngine.NightSkyGameInstance|SetFighterRunner _asbp_night_sky_game_instance "Multiplayer")
  (bind _foundwidgets (Widget|GetAllWidgetsOfClass "/Game/NightSkyEngine/UI/Online/WBP_LobbyList.WBP_LobbyList_C" false))
  (Widget|Panel|ClearChildren (Variables|/Game/NightSkyEngine/UI/Online/WBP_LobbyList.WBP_LobbyList_C|GetLobbyList (Utilities|Array|Get(acopy) _foundwidgets)))
  (Class|NSESessionSubsystem|FindSessions (Subsystems|GetNSESessionSubsystem) 100 false))

(event Custom|PushMenu
  (params (ActivatableWidgetClass :type Common%20Activatable%20Widget%20Class%20Reference))
  (Default|PushMenu (Variables|Default|GetUIBase) ActivatableWidgetClass))

(event Custom|PushModal
  (params (ActivatableWidgetClass :type Common%20Activatable%20Widget%20Class%20Reference))
  (Default|PushModal (Variables|Default|GetUIBase) ActivatableWidgetClass))

(event EventBeginPlay
  (EventDispatchers|AssignOnFindSessionsCompleteEvent (Subsystems|GetNSESessionSubsystem) (delegate Custom|OnFindSessionsCompleteEvent))
  (Utilities|FlowControl|DelayUntilNextFrame)
  (Input|AddMappingContext (PlayerController|LocalPlayerSubsystems|GetEnhancedInputLocalPlayerSubsystem) "/Game/NightSkyEngine/Shared/Input/Menu/IMC_Menu.IMC_Menu" 0 "(bIgnoreAllPressedKeysUntilRelease=True,bForceImmediately=False,bNotifyUserSettings=False)"))

(fn ConstructionScript)