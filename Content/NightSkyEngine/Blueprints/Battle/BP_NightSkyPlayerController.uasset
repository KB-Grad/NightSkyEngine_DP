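; Battle player controller for NightSkyEngine that starts in game-only input and bridges UI events to its UIBase widget.
; Opening the pause menu pushes WBP_PauseMenu as a modal, and prompt and modal requests are forwarded to UIBase.
; Closing the pause or match-end menu deactivates the prompt stack's active widget and restores game input.
; Closing pause also clears PauseGame on the NightSkyGameState.
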(event Custom|PushPrompt
  (params (PromptText :type Text) (PromptOwner :type WBP%20Base%20Activatable%20Widget%20Object%20Reference) (PromptIndex :type Integer))
  (Default|PushPrompt (Variables|Default|GetUIBase) PromptText PromptOwner PromptIndex))

(event Custom|PushModal
  (params (ActivatableWidgetClass :type Common%20Activatable%20Widget%20Class%20Reference))
  (Default|PushModal (Variables|Default|GetUIBase) ActivatableWidgetClass))

(event EventBeginPlay
  (Input|SetInputModeGameOnly self false))

(event EventTick
  (params (DeltaSeconds :type Float%20%28single-precision%29)))

(event EventOpenPauseMenu
  (CallFunction|PushModal "/Game/NightSkyEngine/UI/Battle/WBP_PauseMenu.WBP_PauseMenu_C"))

(event EventClosePauseMenu
  (CallFunction|ClosePauseMenuBP))

(fn ConstructionScript)

(fn ClosePauseMenuBP
  (bind _aswbp_pause_menu (Utilities|Casting|CastToWBP_PauseMenu (Class|CommonActivatableWidgetContainerBase|GetActiveWidget (Variables|/Game/NightSkyEngine/UI/Battle/WBP_BattleBase.WBP_BattleBase_C|GetPromptStack (Variables|Default|GetUIBase))))
    (:then
      (Class|CommonActivatableWidget|DeactivateWidget _aswbp_pause_menu)
      (Input|SetInputModeGameOnly self false)
      (Variables|Default|SetbShowMouseCursor false))
    (:CastFailed
      _))
  (bind _asnight_sky_game_state (Utilities|Casting|CastToNightSkyGameState (Game|GetGameState)))
  (Variables|/Script/NightSkyEngine.NightSkyGameState|SetbPauseGame _asnight_sky_game_state false))

(fn CloseMatchEndMenuBP
  (Class|CommonActivatableWidget|DeactivateWidget (Class|CommonActivatableWidgetContainerBase|GetActiveWidget (Variables|/Game/NightSkyEngine/UI/Battle/WBP_BattleBase.WBP_BattleBase_C|GetPromptStack (Variables|Default|GetUIBase))))
  (Input|SetInputModeGameOnly self false)
  (Variables|Default|SetbShowMouseCursor false))