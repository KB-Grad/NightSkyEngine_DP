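; Battle game state Blueprint for NightSkyEngine that sets up the match HUD, local players and UI.
; On BeginPlay it spawns the battle HUD actor, creates an extra player outside training, CPU battle and multiplayer, then adds a battle base widget for each player controller.
; It pushes the match-end modal on the first controller and copies the battle state's ortho blend value into the character material parameter collection every tick.
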(event EventBeginPlay
  (bind _returnvalue (Game|SpawnActorfromClass "/Game/NightSkyEngine/Blueprints/Battle/BP_NightSkyBattleHudActor.BP_NightSkyBattleHudActor_C" (Math|Transform|MakeTransform "0, 0, 0" "0.000000,90.000000,0.000000" "1.000000,1.000000,1.000000") "Undefined" "MultiplyWithRoot" 0 0))
  (Variables|Default|SetBattleHudActor _returnvalue)
  (bind _asbp_night_sky_game_instance (Utilities|Casting|CastToBP_NightSkyGameInstance (Game|GetGameInstance)))
  (if (and (not (or (Variables|/Script/NightSkyEngine.NightSkyGameInstance|GetIsTraining _asbp_night_sky_game_instance) (Variables|/Script/NightSkyEngine.NightSkyGameInstance|GetIsCPUBattle _asbp_night_sky_game_instance))) (Utilities|Enum|NotEqual(Enum) (Variables|/Script/NightSkyEngine.NightSkyGameInstance|GetFighterRunner _asbp_night_sky_game_instance) "Multiplayer"))
    (Class|GameplayStatics|CreatePlayer -1))
  (bind _outactors (Actor|GetAllActorsOfClass "/Game/NightSkyEngine/Blueprints/Battle/BP_NightSkyPlayerController.BP_NightSkyPlayerController_C"))
  (for _array_element _outactors
    (CallFunction|InitBaseUI _array_element)))

(event EventTick
  (params (DeltaSeconds :type Float%20%28single-precision%29))
  (Rendering|Material|SetScalarParameterValue "/Game/NightSkyEngine/Shared/ParameterCollections/MPC_Chara.MPC_Chara" "OrthoBlendActive" (Utilities|Struct|BreakBattleState (Variables|Default|GetBattleState)) :!class /Script/Engine.KismetMaterialLibrary))

(event EventEndMatchBP
  (bind _asbp_night_sky_player_controller (Utilities|Casting|CastToBP_NightSkyPlayerController (Game|GetPlayerController 0)))
  (Default|PushModal _asbp_night_sky_player_controller "/Game/NightSkyEngine/UI/Battle/WBP_MatchEnd.WBP_MatchEnd_C"))

(fn ConstructionScript)

(fn InitBaseUI
  (params (PlayerController :type BP%20Night%20Sky%20Player%20Controller%20Object%20Reference))
  (bind _returnvalue (UserInterface|CreateWidget "/Game/NightSkyEngine/UI/Battle/WBP_BattleBase.WBP_BattleBase_C" PlayerController))
  (Utilities|IsValid _returnvalue
    (:Is%20Valid
      (bind _output_get (Variables|/Game/NightSkyEngine/Blueprints/Battle/BP_NightSkyPlayerController.BP_NightSkyPlayerController_C|SetUIBase PlayerController _returnvalue))
      (UserInterface|Viewport|AddtoViewport _output_get 0))))