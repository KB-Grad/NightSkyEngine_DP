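; Battle HUD actor for NightSkyEngine that shows the top and bottom HUD widgets through widget components in the world.
; BeginPlay creates both widgets and assigns them to their components.
; Every tick, AdjustWidget pins the top component a fixed distance ahead of the camera, matches its rotation, and scales it by the half-FOV tangent with mirrored axes, keeping its apparent size constant.
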(event EventBeginPlay
  (bind _returnvalue (UserInterface|CreateWidget "/Game/NightSkyEngine/UI/Battle/WBP_BattleHudTop.WBP_BattleHudTop_C"))
  (bind _output_get (Variables|Default|SetTopWidget _returnvalue))
  (UserInterface|SetWidget (Variables|Default|GetBattleHudTop) _output_get)
  (bind _returnvalue_2 (UserInterface|CreateWidget "/Game/NightSkyEngine/UI/Battle/WBP_BattleHudBottom.WBP_BattleHudBottom_C"))
  (bind _output_get_2 (Variables|Default|SetBottomWidget _returnvalue_2))
  (UserInterface|SetWidget (Variables|Default|GetBattleHudBottom) _output_get_2))

(event EventTick
  (params (DeltaSeconds :type Float%20%28single-precision%29))
  (CallFunction|AdjustWidget))

(fn ConstructionScript)

(fn AdjustWidget
  (bind _returnvalue (Game|GetPlayerCameraManager 0))
  (bind _battlehudtop (Variables|Default|GetBattleHudTop))
  (bind _returnvalue_2 (Camera|GetFOVAngle _returnvalue))
  (bind _returnvalue_3 (Camera|GetCameraRotation _returnvalue))
  (bind _returnvalue_4 (* _returnvalue_2 0.5))
  (bind _returnvalue_5 (Math|Trig|Tan(Degrees) _returnvalue_4))
  (bind _returnvalue_6 (* _returnvalue_5 1.125))
  (Transformation|SetRelativeScale3D _battlehudtop (Math|Vector|MakeVector -1.0 (* _returnvalue_6 -1.0) _returnvalue_6))
  (Transformation|SetWorldLocation _battlehudtop (+ (Camera|GetCameraLocation _returnvalue) (* (Math|Rotator|GetRotationXVector _returnvalue_3) 1.08e+03)) false false)
  (Transformation|SetWorldRotation _battlehudtop _returnvalue_3 false false))