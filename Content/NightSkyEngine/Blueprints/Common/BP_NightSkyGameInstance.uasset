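; BP_NightSkyGameInstance is the game instance Blueprint that handles online session setup, replay search results and team list setup for battles.
; On Init it logs in through the NSE session subsystem, and HostSession creates a two-connection non-LAN session when the instance is host.
; Completed replay searches are forwarded to the first WBP_ReplayMenu widget.
; InitPlayerList clears and resizes both players' character and color arrays to their team sizes.
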(event Custom|HostSession
  (if (Variables|Default|GetIsHost)
    (Class|NSESessionSubsystem|CreateSession (Subsystems|GetNSESessionSubsystem) 2 false)))

(event EventOnFindReplaysComplete
  (params (AllReplays :type Array%20of%20Replay%20Save%20Info%20Object%20References))
  (Utilities|Casting|CastToBP_MenuPlayerController (Game|GetPlayerController 0))
  (bind _foundwidgets (Widget|GetAllWidgetsOfClass "/Game/NightSkyEngine/UI/Replay/WBP_ReplayMenu.WBP_ReplayMenu_C" false))
  (Default|OnFindReplays (Utilities|Array|Get(acopy) _foundwidgets) AllReplays))

(event EventInit
  (Class|NSESessionSubsystem|Login (Subsystems|GetNSESessionSubsystem)))

(fn InitPlayerList
  (bind _battledata (Variables|Default|GetBattleData))
  (bind (_playerlistp1 _playerlistp2 _colorindicesp1 _colorindicesp2) (Utilities|Struct|BreakBattleData _battledata))
  (Utilities|Array|Clear _playerlistp1)
  (Utilities|Array|Resize _playerlistp1 (Variables|Default|GetTeamSizeP1))
  (Utilities|Array|Clear _playerlistp2)
  (Utilities|Array|Resize _playerlistp2 (Variables|Default|GetTeamSizeP2))
  (Utilities|Array|Clear _colorindicesp1)
  (Utilities|Array|Resize _colorindicesp1 (Variables|Default|GetTeamSizeP1))
  (Utilities|Array|Clear _colorindicesp2)
  (Utilities|Array|Resize _colorindicesp2 (Variables|Default|GetTeamSizeP2)))